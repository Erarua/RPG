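; Gameplay ability for a player-targeted AOE lightning strike, placed with a ground-trace decal.
; While a looping targeting montage plays, it waits for confirmation, or an input press to cancel, and raises the input mapping priority until it ends.
; Confirming commits the ability, shows an indicator cue and plays the trigger montage.
; That montage's event fires the lightning cue and server-side sphere-trace damage, applied once per actor via SetByCaller effect.
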(event Custom|LoopTargetingAnimation
  (|PlayMontageandWaitProxy "None" "/Game/Animations/Staff/Montage_AOE_Targeting.Montage_AOE_Targeting" 1.0 "None" true 1.0 0.0 false
    (:OnBlendOut
      (if (Variables|Default|GetIsWaitingTargetData)
        (CallFunction|LoopTargetingAnimation)))
    (:OnInterrupted
      (if (Variables|Default|GetIsWaitingTargetData)
        (Ability|EndAbility)))))

(event Custom|ConfirmStrike
  (bind _returnvalue (Ability|CommitAbility))
  (if _returnvalue
    (Class|GameplayAbility|AddGameplayCuewithParams "(TagName=\"GameplayCue.AOEIndicator\")" (Ability|GameplayCue|MakeGameplayCueParameters :RawMagnitude (* (Variables|Default|GetAOERadius) 2.0) :Location (Variables|Default|GetConfirmedAOELocation)) true)
    (|PlayMontageandWaitProxy "None" "/Game/Animations/Staff/Montage_AOE_Trigger.Montage_AOE_Trigger" 1.0 "None" true 1.0 0.0 false
      (:then
        (Ability|Tasks|WaitGameplayEvent "(TagName=\"Event.Montage.Trigger\")" 0
          (:EventReceived
            (Utilities|FlowControl|Delay 0.2)
            (Class|GameplayAbility|ExecuteGameplayCuewithParams "(TagName=\"GameplayCue.LightningBolt\")" (Ability|GameplayCue|MakeGameplayCueParameters :Location (Variables|Default|GetConfirmedAOELocation)))
            (CallFunction|AOEDamage)
            (GameplayCue|RemoveGameplayCue "(TagName=\"GameplayCue.AOEIndicator\")"))))
      (:OnCompleted
        (Ability|EndAbility :!label _label))
      (:OnInterrupted
        (goto _label)))
    (else
      (Ability|EndAbility))))

(event Custom|AOEDamage
  (bind _confirmedaoelocation (Variables|Default|GetConfirmedAOELocation))
  (Ability|HasAuthority
    (:True
      (bind _outhits (Collision|MultiSphereTraceForObjects _confirmedaoelocation _confirmedaoelocation (Variables|Default|GetAOERadius) (Utilities|Array|MakeArray "ObjectTypeQuery3") false (Utilities|Array|MakeArray (Ability|GetAvatarActorfromActorInfo)) "ForDuration" true "(R=1.000000,G=0.000000,B=0.000000,A=1.000000)" "(R=0.000000,G=1.000000,B=0.000000,A=1.000000)" 1.0))
      (Utilities|Array|Clear (Variables|Default|GetHitActors))
      (for _array_element _outhits
        (if (not (Utilities|Array|ContainsItem (Variables|Default|GetHitActors) (.HitActor (Collision|BreakHitResult _array_element))))
          (Utilities|Array|AddUnique (Variables|Default|GetHitActors) (.HitActor (Collision|BreakHitResult _array_element)))
          (Utilities|IsValid (Ability|GetAbilitySystemComponent (.HitActor (Collision|BreakHitResult _array_element)))
            (:Is%20Valid
              (bind _returnvalue (Ability|GameplayEffect|AssignTagSetbyCallerMagnitude (Ability|MakeOutgoingGameplayEffectSpec "/Game/GameplayAbilitySystem/Effects/GE_Damege_Instant.GE_Damege_Instant_C") "(TagName=\"Data.Damage\")" (Variables|Default|GetDamageMagnitude)))
              (GameplayEffects|ApplyGameplayEffectSpecToTarget (Ability|GetAbilitySystemComponent (Ability|GetAvatarActorfromActorInfo)) _returnvalue (Ability|GetAbilitySystemComponent (.HitActor (Collision|BreakHitResult _array_element)))))))))))

(event Custom|WaitCancel
  (Ability|Tasks|WaitInputPress false
    (:OnPress
      (Ability|EndAbility))))

(event Ability|EventActivateAbility
  (CallFunction|WaitCancel)
  (CallFunction|LoopTargetingAnimation)
  (Variables|Default|SetIsWaitingTargetData true)
  (Input|AddMappingContext (PlayerController|LocalPlayerSubsystems|GetEnhancedInputLocalPlayerSubsystem (.PlayerController (Utilities|Struct|BreakGameplayAbilityActorInfo (Ability|GetActorInfo)))) "/Game/Input/IMC_Default.IMC_Default" 1 "(bIgnoreAllPressedKeysUntilRelease=True,bForceImmediately=False,bNotifyUserSettings=False)")
  (bind _data (|WaitTargetData :ConfirmationType "UserConfirmed" :Class "/Game/GameplayAbilitySystem/TargetActors/GATarget_GroundTrace_Decal.GATarget_GroundTrace_Decal_C" :Decal "/Game/Decals/Decal_AOE.Decal_AOE" :DecalSize (* (Variables|Default|GetAOERadius) 2.0) :StartLocation (Class|GameplayAbility|MakeTargetLocationInfofromOwnerActor) :ReticleClass 0)
    (:ValidData
      (Variables|Default|SetIsWaitingTargetData false)
      (Variables|Default|SetConfirmedAOELocation (.Location (Collision|BreakHitResult (Ability|TargetData|GetHitResultfromTargetData _data))))
      (CallFunction|ConfirmStrike))))

(event Ability|EventOnEndAbility
  (params (bWasCancelled :type Boolean))
  (Input|AddMappingContext (PlayerController|LocalPlayerSubsystems|GetEnhancedInputLocalPlayerSubsystem (.PlayerController (Utilities|Struct|BreakGameplayAbilityActorInfo (Ability|GetActorInfo)))) "/Game/Input/IMC_Default.IMC_Default" 0 "(bIgnoreAllPressedKeysUntilRelease=True,bForceImmediately=False,bNotifyUserSettings=False)"))