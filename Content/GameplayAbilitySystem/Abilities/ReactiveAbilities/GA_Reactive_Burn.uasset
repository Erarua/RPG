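; Reactive burn ability that applies a damage-over-time debuff to targets its owner hits.
; Activated from a gameplay event, it runs on authority only and checks that the owner is the instigator, the tag is Event.Hit and the target has an ability system component.
; The effect spec comes from DebuffSettings, with duration and SetByCaller Data.Damage overridden before application.
; Debug prints remain, and the graph never calls EndAbility.
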(event Ability|EventActivateAbilityFromEvent
  (params (EventData :type Gameplay%20Event%20Data%20Structure%20%28by%20ref%29))
  (bind (_eventtag _instigator _target) (Utilities|Struct|BreakGameplayEventData EventData))
  (Development|PrintString "Hello")
  (Ability|HasAuthority
    (:True
      (Development|PrintString "GE_Burn_Auth")
      (if (and (== (Ability|GetOwningActorfromActorInfo) _instigator) (== _eventtag "(TagName=\"Event.Hit\")"))
        (Utilities|IsValid (Ability|GetAbilitySystemComponent _target)
          (:Is%20Valid
            (bind _outspec (CallFunction|ModifyEffectSpecHandleBeforeApplied (Ability|MakeOutgoingGameplayEffectSpec (Variables|/Game/GameplayAbilitySystem/DebuffDataAssets/PDA_DebuffSettings.PDA_DebuffSettings_C|GetDebuffEffect (Variables|Default|GetDebuffSettings)))))
            (GameplayEffects|ApplyGameplayEffectSpecToTarget _outspec (Ability|TargetData|AbilityTargetDatafromActor _target))))))))

(fn ModifyEffectSpecHandleBeforeApplied
  (params (InSpec :type Gameplay%20Effect%20Spec%20Handle%20Structure))
  (bind _returnvalue (Ability|GameplayEffect|SetDuration InSpec (Variables|/Game/GameplayAbilitySystem/DebuffDataAssets/PDA_DebuffSettings.PDA_DebuffSettings_C|GetDebuffDuration (Variables|Default|GetDebuffSettings))))
  (bind _returnvalue_2 (Ability|GameplayEffect|AssignTagSetbyCallerMagnitude _returnvalue "(TagName=\"Data.Damage\")" (Variables|/Game/GameplayAbilitySystem/DebuffDataAssets/PDA_DebuffSettings.PDA_DebuffSettings_C|GetDamagePerSecond (Variables|Default|GetDebuffSettings))))
  (return _returnvalue_2))