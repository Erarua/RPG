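; Base Gameplay Ability that fires a projectile, with configurable montage, projectile class, speed and damage effect.
; It plays the shoot montage, waits for the Event.ShootProjectile event, then takes an instant line-trace target point.
; The projectile spawns only on authority at the equipped weapon's spawn point, falling back to actor location, and carries a SetByCaller damage spec.
; The ability ends when the montage completes, is interrupted or is cancelled.
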(event Ability|EventActivateAbility
  (|PlayMontageandWaitProxy "None" (Variables|Default|GetShootMontage) 1.0 "None" true 1.0 0.0 false
    (:then
      (Ability|Tasks|WaitGameplayEvent "(TagName=\"Event.ShootProjectile\")" 0
        (:EventReceived
          (bind _data (|WaitTargetData :ConfirmationType "Instant" :Class "/Script/GameplayAbilities.GameplayAbilityTargetActor_SingleLineTrace" :TraceProfile "(Name=\"NoCollision\")" :StartLocation (Class|GameplayAbility|MakeTargetLocationInfofromOwnerActor) :ReticleClass 0)
            (:ValidData
              (bind _returnvalue (Ability|GameplayEffect|AssignTagSetbyCallerMagnitude (Ability|MakeOutgoingGameplayEffectSpec (Variables|GameplayEffect|GetDamageEffectClass)) "(TagName=\"Data.Damage\")" (Variables|GameplayEffect|GetDamageMagnitude)))
              (bind _location (CallFunction|GetSpawnLocation))
              (|SpawnActor 0 _location "0, 0, 0" (Variables|ProjectileSettings|GetProjectileClass) true (Variables|ProjectileSettings|GetProjectileSpeed) (Class|AbilitySystemBlueprintLibrary|GetTargetDataEndPoint _data) _returnvalue (.AsPawn (Utilities|Casting|CastToPawn (Ability|GetAvatarActorfromActorInfo)))))))))
    (:OnCompleted
      (Ability|EndAbility :!label _label))
    (:OnInterrupted
      (goto _label))
    (:OnCancelled
      (goto _label))))

(event Ability|EventOnEndAbility
  (params (bWasCancelled :type Boolean)))

(fn GetSpawnLocation
  (bind _returnvalue (Ability|GetAvatarActorfromActorInfo))
  (bind _returnvalue_2 (Actor|GetComponentbyClass _returnvalue "/Game/Weapons/WeaponsManagementComponent.WeaponsManagementComponent_C"))
  (Utilities|IsValid _returnvalue_2
    (:Is%20Valid
      (bind _equippedweapon (Variables|/Game/Weapons/WeaponsManagementComponent.WeaponsManagementComponent_C|GetEquippedWeapon _returnvalue_2)
        (:then
          (bind _location (Default|GetSpawnPointLocation _equippedweapon))
          (if (Utilities|Operators|NotEqual(!=) :A _location)
            (return _location)
            (else
              _)))
        (:else
          _)))
    (:Is%20Not%20Valid
      _))
  (return (Transformation|GetActorLocation (Ability|GetAvatarActorfromActorInfo))))